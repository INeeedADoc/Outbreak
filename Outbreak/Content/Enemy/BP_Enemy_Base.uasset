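; Base enemy that pursues the player, takes damage and dies.
; Actor tags choose between a repeating AIMoveTo chase (Enemy_1/2) and a move to a unit direction vector, retried after delayed success (Enemy_3).
; Damage lowers Health, pausing movement for random hit montages or playing a death montage.
; Death calls the player's InteractPointsMessage, removes the capsule and destroys the actor after a delay; a tag-based death branch is unwired.
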(event `self.ReceiveBeginPlay`
  ; Chase Player
  (bind _asbp_first_person_character (cast `/Game/FirstPerson/Blueprints/BP_FirstPersonCharacter` (`GameplayStatics.GetPlayerCharacter` 0)))
  (set `self.As BP First Person Character` _asbp_first_person_character)
  (if (`self.ActorHasTag` "Enemy_1")
    (`self.Chase_Player` (`self.As BP First Person Character`) :!label _label)
    (elif (`self.ActorHasTag` "Enemy_2")
      (goto _label)
      (elif (`self.ActorHasTag` "Enemy_3")
        (`self.Enemy_3_Movement` self (`self.As BP First Person Character`))))))

(event `Chase_Player`
  (params (Target :type "Pawn Object Reference"))
  ; Chase Player
  (if (not (`self.Dead?`))
    (`|AIMoveTo` self (0.0 0.0 0.0) Target 30.0
      (:`OnSuccess`
        (`KismetSystemLibrary.Delay` 0.1))
      (:`OnFail`
        _))
    (`self.Chase_Player` Target)))

(event `Enemy_3_Movement`
  (params (Enemy :type "Pawn Object Reference") (Target :type "Pawn Object Reference"))
  (if (not (`self.Dead?`))
    (`|AIMoveTo` self (`KismetMathLibrary.GetDirectionUnitVector` (`SceneComponent.K2_GetComponentLocation` (`Actor.RootComponent` Enemy)) (`SceneComponent.K2_GetComponentLocation` (`Actor.RootComponent` Target))) null 30.0
      (:`OnSuccess`
        (`KismetSystemLibrary.Delay` 5.0)
        (`self.Enemy_3_Movement` self (`self.As BP First Person Character`))))))

(event `self.ReceiveAnyDamage`
  (params (Damage :type "Float (single-precision)") (DamageType :type "DamageType Object Reference") (InstigatedBy :type "Controller Object Reference") (DamageCauser :type "Actor Object Reference"))
  (bind _health (`self.Health`))
  ; Death/Hit + Animation
  (if (not (`self.Dead?`))
    (set `self.Health` (- _health Damage))
    (if (<= _health 0.0)
      (`CharacterMovementComponent.DisableMovement` (`self.CharacterMovement`))
      (set `self.Dead?` true)
      (`self.PlayAnimMontage` (select `int` (`KismetMathLibrary.RandomInteger` 2) :`0` "/Game/Enemy/Assets/Death1_Montage.Death1_Montage" :`1` "/Game/Enemy/Assets/Death2_Montage.Death2_Montage" :`2` "/Game/Enemy/Assets/Death3_Montage.Death3_Montage" :!type "AnimMontage Object Reference"))
      (`self.Enemy is Dead`)
      (else
        (`CharacterMovementComponent.DisableMovement` (`self.CharacterMovement`))
        (bind _returnvalue (`self.PlayAnimMontage` (select `int` (`KismetMathLibrary.RandomInteger` 2) :`0` "/Game/Enemy/Assets/Hit1_Montage.Hit1_Montage" :`1` "/Game/Enemy/Assets/Hit2_Montage.Hit2_Montage" :`2` "/Game/Enemy/Assets/Hit3_Montage.Hit3_Montage" :!type "AnimMontage Object Reference")))
        (`KismetSystemLibrary.Delay` _returnvalue)
        (if (not (`self.Dead?`))
          (`CharacterMovementComponent.SetMovementMode` (`self.CharacterMovement`) "MOVE_Walking" 0))))))

(event `Enemy is Dead`
  ; Death/Hit + Animation
  (message `/Game/FirstPerson/InteractInterface.InteractPoints` (`GameplayStatics.GetPlayerCharacter` 0) :!label _label_2)
  (`ActorComponent.K2_DestroyComponent` (`self.CapsuleComponent`))
  (`KismetSystemLibrary.Delay` 10.0)
  (`self.K2_DestroyActor`)
  (goto _label_2))

(fn `UserConstructionScript`)