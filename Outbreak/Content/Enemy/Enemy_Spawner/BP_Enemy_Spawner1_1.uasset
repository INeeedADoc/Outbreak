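; Enemy spawner actor that, once activated, spawns a queue of enemy classes one at a time at its own transform.
; An activation event sets the active flag and calls the spawn event.
; The spawn event spawns the first class in the queue, removes it, waits a spawn delay and calls itself again until the queue is empty.
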(event `self.ReceiveBeginPlay`)

(event `Spawn Enemys1_1`
  (params (EnemyQueu :type "Array of /Game/Enemy/BP_Enemy_Base Class Reference"))
  (if (`self.IsActive?`)
    (if (`KismetArrayLibrary.Array_IsValidIndex` EnemyQueu)
      (`|SpawnActorFromClass` (`|GetArrayItem` EnemyQueu) (`self.GetTransform`) "Undefined" "MultiplyWithRoot" null null)
      (`KismetArrayLibrary.Array_Remove` EnemyQueu)
      (`KismetSystemLibrary.Delay` (`self.Spawn_Delay`))
      (`self.Spawn Enemys1_1` EnemyQueu))))

(event `/Game/FirstPerson/InteractInterface.ActivateSpawner1_1`
  (set `self.IsActive?` true)
  (`self.Spawn Enemys1_1` _))

(fn `UserConstructionScript`)