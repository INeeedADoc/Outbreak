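; Spawner actor that produces waves of enemies at its own transform for as long as it runs.
; BeginPlay starts SpawnEnemys, which spawns EnemyCount actors of the chosen class, waits SpawnDelay, then calls itself to loop indefinitely.
; Each wave selects between Enemy_1 and Enemy_2 via RandomInteger(1), which only returns 0, so Enemy_1 is always chosen.
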(event `self.ReceiveBeginPlay`
  (`self.Spawn Enemys` (select `int` (`KismetMathLibrary.RandomInteger` 1) :`0` "/Game/Enemy/Enemy_1/Enemy_1.Enemy_1_C" :`1` "/Game/Enemy/Enemy_2/Enemy_2.Enemy_2_C" :!type "Actor Class Reference") (`self.GetTransform`) (`self.Enemy Count`)))

(event `Spawn Enemys`
  (params (Enemy_Type :type "Actor Class Reference") (SpawnTransform :type "Transform Structure") (Enemy_Count :type Integer))
  (for _ (range Enemy_Count)
    (`|SpawnActorFromClass` Enemy_Type SpawnTransform "Undefined" "MultiplyWithRoot" null null))
  (`KismetSystemLibrary.Delay` (`self.Spawn_Delay`))
  (`self.Spawn Enemys` (select `int` (`KismetMathLibrary.RandomInteger` 1) :`0` "/Game/Enemy/Enemy_1/Enemy_1.Enemy_1_C" :`1` "/Game/Enemy/Enemy_2/Enemy_2.Enemy_2_C" :!type "Actor Class Reference") (`self.GetTransform`) (`self.Enemy Count`)))

(fn `UserConstructionScript`)